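; Weather Blueprint that darkens the sky from bright blue to overcast grey when W is pressed.
; If SkyRef is valid, a timeline plays from the start and drives lerps on the referenced sky's material.
; It blends zenith, horizon and cloud colours towards dark greys.
; It also raises a scalar parameter, but that parameter's name is None, and no path reverses the change.
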(event `Key|W`
  (params (Key :type "Key Structure"))
  (bind _sky_material (`/Engine/EngineSky/BP_Sky_Sphere.Sky material` (`self.SkyRef`)))
  (:`Pressed`
    (if (`KismetSystemLibrary.IsValid` (`self.SkyRef`))
      (bind (_direction _newtrack_0) (`Timeline|Timeline_0` :!via `PlayFromStart`)
        (:`Update`
          (`MaterialInstanceDynamic.SetVectorParameterValue` _sky_material "Zenith Color" (`KismetMathLibrary.LinearColorLerp` (struct :`R` 0.034046 :`G` 0.109247 :`B` 0.295 :`A` 1.0) (struct :`R` 0.072917 :`G` 0.072917 :`B` 0.072917 :`A` 1.0) _newtrack_0))
          (`MaterialInstanceDynamic.SetVectorParameterValue` _sky_material "Horizon Color" (`KismetMathLibrary.LinearColorLerp` (struct :`R` 1.979559 :`G` 2.586644 :`B` 3.0 :`A` 1.0) (struct :`R` 0.041667 :`G` 0.041667 :`B` 0.041667 :`A` 1.0) _newtrack_0))
          (`MaterialInstanceDynamic.SetVectorParameterValue` _sky_material "Cloud Color" (`KismetMathLibrary.LinearColorLerp` (struct :`R` 2.6875 :`G` 2.807969 :`B` 3.0 :`A` 1.0) (struct :`R` 0.015625 :`G` 0.015625 :`B` 0.015625 :`A` 1.0) _newtrack_0))
          (`MaterialInstanceDynamic.SetScalarParameterValue` _sky_material "None" (`KismetMathLibrary.Lerp` 1.2 5.0 _newtrack_0)))))))

(fn `UserConstructionScript`)