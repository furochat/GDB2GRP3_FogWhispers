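; BP_SpecialKey is a collectible key item that the player picks up by interacting with it.
; The construction script sets the key mesh material from KeyType, with copper, silver and gold variants for the three key tiers.
; On interaction it adds KeyType to the DefaultCharacter's OwnedKeys, flags itself as picked up, plays a collect sound at the world origin and destroys itself.
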(event `/Game/InterfaceAndUI/Interfaces/Interact_Interface.OnInteraction`
  (params (Player :type "/Game/Actors/Characters/DefaultCharacter Object Reference"))
  (bind _asdefault_character (cast `/Game/Actors/Characters/DefaultCharacter` Player))
  (`KismetArrayLibrary.Array_Add` (`/Game/Actors/Characters/DefaultCharacter.OwnedKeys` _asdefault_character) (`self.KeyType`))
  (set `self.KeyPickedUP` true)
  (`GameplayStatics.PlaySoundAtLocation` "/Game/Assets/SFX/Collect.Collect" (0.0 0.0 0.0) (struct) 1.0 1.0 0.0 null null null)
  (`self.K2_DestroyActor`))

(fn `UserConstructionScript`
  (`PrimitiveComponent.SetMaterial` (`self.Key`) 0 (select `/Game/Assets/Items/SceneObjects/EKeyTypes` (`self.KeyType`) :`NewEnumerator0` "/Game/Assets/Materials/Object/M_KeyType.M_KeyType" :`NewEnumerator1` "/Game/Assets/Materials/Object/M_CopperKey_Inst.M_CopperKey_Inst" :`NewEnumerator2` "/Game/Assets/Materials/Object/M_SilverKey_Inst.M_SilverKey_Inst" :`NewEnumerator3` "/Game/Assets/Materials/Object/M_GoldKey_Inst.M_GoldKey_Inst" :!type "MaterialInterface Object Reference")))