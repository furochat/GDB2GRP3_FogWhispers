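; Interactable door that swings on a timeline-driven yaw rotation and is gated by three key actors, despite the DoubleKey name.
; On interaction, a player key matching the first required type triggers checks of each key actor's pickup flag.
; If all flags and Open are true, it opens, removes that key and syncs keys to IslandGameInstance; otherwise it closes.
; An unconnected HasKey branch holds the locked sound.
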(event `Open`
  (set `self.Open?` true)
  (bind (_direction _door_track) (`Timeline|Timeline_0` :!label _label)
    (:`Update`
      (`SceneComponent.K2_SetRelativeRotation` (`self.StaticMesh`) (`KismetMathLibrary.MakeRotator` 0.0 0.0 (`KismetMathLibrary.Lerp` (`self.CloseAngle`) (`self.OpenAngle`) _door_track)) false false))))

(event `Close`
  (set `self.Open?` false)
  (goto _label :!via `Reverse`))

(event `/Game/InterfaceAndUI/Interfaces/Interact_Interface.OnInteraction`
  (params (Player :type "/Game/Actors/Characters/DefaultCharacter Object Reference"))
  (bind _asdefault_character (cast `/Game/Actors/Characters/DefaultCharacter` Player))
  (bind _ownedkeys (`/Game/Actors/Characters/DefaultCharacter.OwnedKeys` _asdefault_character))
  (for (_array_element _array_index) _ownedkeys
    (if (`|EnumEquality` _array_element (`|GetArrayItem` (`self.RecquiredKeyType`)))
      (if true
        (`|ExecutionSequence`
          (:`then_0`
            (bind _output_get (set `self.KeyTwoPicked` (`/Game/Assets/Items/InventoryItems/BP_SpecialKey.KeyPickedUP` (`self.KeyTwo`))))
            (if (and (stale _output_get_2) _output_get (stale _output_get_3) (`self.Open?`)) :!label _label_2
              (set `self.Open?` true)
              (`self.Open`)
              (`KismetArrayLibrary.Array_Remove` _ownedkeys _array_index)
              (bind _asisland_game_instance (cast `/Game/Actors/Logics/Logic_CharacterSelection/IslandGameInstance` (`GameplayStatics.GetGameInstance`)))
              (set `/Game/Actors/Logics/Logic_CharacterSelection/IslandGameInstance.PlayerKeys` _ownedkeys _asisland_game_instance)
              (else
                (set `self.Open?` false)
                (`self.Close`))))
          (:`then_1`
            (bind _output_get_2 (set `self.KeyOnePicked` (`/Game/Assets/Items/InventoryItems/BP_SpecialKey.KeyPickedUP` (`self.KeyOne`)))))
          (:`then_2`
            (bind _output_get_3 (set `self.KeyTreePicked` (`/Game/Assets/Items/InventoryItems/BP_SpecialKey.KeyPickedUP` (`self.KeyThree`))))
            (goto _label_2)))))))

(fn `UserConstructionScript`)