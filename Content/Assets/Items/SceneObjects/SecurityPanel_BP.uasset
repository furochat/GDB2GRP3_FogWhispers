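; Security panel actor that guards a strongbox with a password keypad.
; UseKeypad opens a PasswordScreenUI widget that holds a back-reference to the panel, switches input to UI-only and shows the mouse cursor.
; CorrectPassword opens the referenced strongbox door and spawns a special key child actor at a stored transform.
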(event `Use Keypad`
  (bind _returnvalue (`GameplayStatics.GetPlayerController` 0))
  (bind _returnvalue_2 (`|CreateWidget` "/Game/InterfaceAndUI/UserInterface/PassWordScreenUI.PasswordScreenUI_C"))
  (set `/Game/InterfaceAndUI/UserInterface/PassWordScreenUI.SecurityPanelBP` self _returnvalue_2)
  (`UserWidget.AddToViewport` _returnvalue_2 0)
  (`WidgetBlueprintLibrary.SetInputMode_UIOnlyEx` _returnvalue null)
  (set `PlayerController.bShowMouseCursor` true _returnvalue))

(event `CorrectPassword`
  (`|ExecutionSequence`
    (:`then_0`
      (`/Game/FirstPersonBP/Props/CoffreFort/BP_CoffreFort.OpenDoor` (`self.StrongBoxDoorBP`)))
    (:`then_1`
      (`|SpawnActorFromClass` "/Game/Assets/Items/InventoryItems/BP_SpecialKey2_Child.BP_SpecialKey2_Child_C" (`self.SpawnTransform`) "Undefined" "OverrideRootScale" null null))))

(fn `UserConstructionScript`)