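; BP_CombinaisonLockDoor is a door scene object, named for a combination lock, that swings open and closed.
; It caches the mesh's world rotation on BeginPlay, then Open plays a timeline that adds a yaw offset to that rotation and Close reverses it.
; Both events print French debug messages; the file itself holds no combination or lock logic.
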(event `self.ReceiveBeginPlay`
  (set `self.DefaultRotation` (`SceneComponent.K2_GetComponentRotation` (`self.StaticMesh`))))

(event `Open`
  (`KismetSystemLibrary.PrintString` "Ouvert")
  (bind (_direction _zaxis) (`Timeline|Timeline_0` :!label _label)
    (:`Update`
      (`SceneComponent.K2_SetWorldRotation` (`self.StaticMesh`) (`KismetMathLibrary.ComposeRotators` (`KismetMathLibrary.MakeRotator` 0.0 0.0 _zaxis) (`self.DefaultRotation`)) false false))))

(event `Close`
  (`KismetSystemLibrary.PrintString` "Se ferme")
  (goto _label :!via `Reverse`))

(fn `UserConstructionScript`)