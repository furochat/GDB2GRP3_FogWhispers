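; Double door that the StrongCharacter_Child player kicks open, swinging only the right leaf (PorteD).
; A box overlap toggles input and a gate while that character is in range.
; The first KickDown press snaps the player to the SkeletalMesh transform, plays a kick montage and drives the door's yaw by timeline.
; A gated FlipFlop open/close timeline also exists, but its DoOnce starts closed and is never reset.
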(event `InputAction|KickDown`
  (params (Key :type "Key Structure"))
  (:`Pressed`
    (`|ExecutionSequence`
      (:`then_0`
        (`/Engine/EditorBlueprintResources/StandardMacros.DoOnce` false
          (:`Completed`
            (bind _asstrong_character_child (cast `/Game/Actors/Characters/StrongCharacter_Child` (`GameplayStatics.GetPlayerCharacter` 0)))
            (`self.K2_SetActorTransform` _asstrong_character_child (`SceneComponent.K2_GetComponentToWorld` (`self.SkeletalMesh`)) false false)
            (`Character.PlayAnimMontage` _asstrong_character_child "/Game/Assets/Models/Mannequin/Animations/Kick/Kicking_Anim_mixamo_com1_Montage.Kicking_Anim_mixamo_com1_Montage" 1.0 "None")
            (bind (_direction _door_kick_track) (`Timeline|Timeline_0`)
              (:`Update`
                (`SceneComponent.K2_SetRelativeRotation` (`self.PorteD`) (`KismetMathLibrary.MakeRotator` 0.0 0.0 (`KismetMathLibrary.Lerp` 0.0 -100.0 _door_kick_track)) false false))))))
      (:`then_1`
        (`/Engine/EditorBlueprintResources/StandardMacros.DoOnce` true
          (:`Completed`
            (`/Engine/EditorBlueprintResources/StandardMacros.Gate` true :!label _label
              (:`Exit`
                (`/Engine/EditorBlueprintResources/StandardMacros.FlipFlop`
                  (:`A`
                    (bind (_direction_2 _open_close_track_right_door) (`Timeline|Right` :!label _label_2)
                      (:`Update`
                        (`SceneComponent.K2_SetRelativeRotation` (`self.PorteD`) (`KismetMathLibrary.MakeRotator` 0.0 0.0 (`KismetMathLibrary.Lerp` 0.0 -100.0 _open_close_track_right_door)) false false))))
                  (:`B`
                    (goto _label_2 :!via `Reverse`)))))))))))

(event `self.Box.OnComponentBeginOverlap`
  (params (OverlappedComponent :type "PrimitiveComponent Object Reference") (OtherActor :type "Actor Object Reference") (OtherComp :type "PrimitiveComponent Object Reference") (OtherBodyIndex :type Integer) (bFromSweep :type Boolean) (SweepResult :type "HitResult Structure (by ref)"))
  (cast `/Game/Actors/Characters/StrongCharacter_Child` OtherActor)
  (`self.EnableInput` (`GameplayStatics.GetPlayerController` 0))
  (goto _label :!via `Open`))

(event `self.Box.OnComponentEndOverlap`
  (params (OverlappedComponent :type "PrimitiveComponent Object Reference") (OtherActor :type "Actor Object Reference") (OtherComp :type "PrimitiveComponent Object Reference") (OtherBodyIndex :type Integer))
  (cast `/Game/Actors/Characters/StrongCharacter_Child` OtherActor)
  (`self.DisableInput` (`GameplayStatics.GetPlayerController` 0))
  (goto _label :!via `Close`))

(fn `UserConstructionScript`)