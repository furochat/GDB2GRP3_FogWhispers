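; BP_LockedDoor is a door that responds to interaction only when the player holds a key matching its KeyChannel.
; OnInteraction checks the key, then calls Open if the Open flag is true and Close otherwise, each re-setting the flag to that same state.
; Open plays and Close reverses the OpenClose timeline, whose track interpolates the static mesh's relative yaw between CloseAngle and OpenAngle.
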(event `/Game/InterfaceAndUI/Interfaces/Interact_Interface.OnInteraction`
  (params (Player :type "/Game/Actors/Characters/DefaultCharacter Object Reference"))
  (`/Engine/EditorBlueprintResources/StandardMacros.IsValid` Player
    (:`Is Valid`
      (if (`/Game/Actors/Characters/DefaultCharacter.HasKey?` Player (`self.KeyChannel`))
        (if (`self.Open?`)
          (`self.Open`)
          (else
            (`self.Close`)))))))

(event `Open`
  (set `self.Open?` true)
  (bind (_direction _door_track) (`Timeline|Open/Close` :!label _label)
    (:`Update`
      (`SceneComponent.K2_SetRelativeRotation` (`self.StaticMesh`) (`KismetMathLibrary.MakeRotator` 0.0 0.0 (`KismetMathLibrary.Lerp` (`self.Close Angle`) (`self.Open Angle`) _door_track)) false false))))

(event `Close`
  (set `self.Open?` false)
  (goto _label :!via `Reverse`))

(fn `UserConstructionScript`)