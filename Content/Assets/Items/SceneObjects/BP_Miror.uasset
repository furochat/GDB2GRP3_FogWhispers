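; BP_Miror is a mirror scene object that drains an AgilityCharacter_Child's mental health while the player is near it.
; FarRange and CloseRange overlaps each run a Delay-based loop gated by a presence flag, with the close one ticking faster.
; Each tick prints the value and sends KillPlayerMessage to the player controller at zero.
; The Box overlap toggles both flags and the PostProcessAgility blend weight, without starting a drain loop itself.
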(event `self.FarRange.OnComponentBeginOverlap`
  (params (OverlappedComponent :type "PrimitiveComponent Object Reference") (OtherActor :type "Actor Object Reference") (OtherComp :type "PrimitiveComponent Object Reference") (OtherBodyIndex :type Integer) (bFromSweep :type Boolean) (SweepResult :type "HitResult Structure (by ref)"))
  (bind _asagility_character_child (cast `/Game/Actors/Characters/AgilityCharacter_Child` OtherActor))
  (set `self.PlayerInLightBox` true)
  (bind _output_get (set `/Game/Actors/Characters/DefaultCharacter.Current Mental Health` (- (`/Game/Actors/Characters/DefaultCharacter.Current Mental Health` _asagility_character_child) 1.0) _asagility_character_child :!label _label))
  (`KismetSystemLibrary.PrintString` (`KismetStringLibrary.Conv_DoubleToString` _output_get))
  (if (<= _output_get 0.0)
    (message `/Game/InterfaceAndUI/Interfaces/Interact_Interface.KillPlayer` (`GameplayStatics.GetPlayerController` 0))
    (else
      (`KismetSystemLibrary.Delay` 3.0)
      (if (`self.PlayerInLightBox`)
        (goto _label)))))

(event `self.FarRange.OnComponentEndOverlap`
  (params (OverlappedComponent :type "PrimitiveComponent Object Reference") (OtherActor :type "Actor Object Reference") (OtherComp :type "PrimitiveComponent Object Reference") (OtherBodyIndex :type Integer))
  (cast `/Game/Actors/Characters/AgilityCharacter_Child` OtherActor)
  (set `self.PlayerInLightBox` false))

(event `self.CloseRange.OnComponentBeginOverlap`
  (params (OverlappedComponent :type "PrimitiveComponent Object Reference") (OtherActor :type "Actor Object Reference") (OtherComp :type "PrimitiveComponent Object Reference") (OtherBodyIndex :type Integer) (bFromSweep :type Boolean) (SweepResult :type "HitResult Structure (by ref)"))
  (bind _asagility_character_child (cast `/Game/Actors/Characters/AgilityCharacter_Child` OtherActor))
  (set `self.PlayerInCloseLightBox` true)
  (bind _output_get (set `/Game/Actors/Characters/DefaultCharacter.Current Mental Health` (- (`/Game/Actors/Characters/DefaultCharacter.Current Mental Health` _asagility_character_child) 1.0) _asagility_character_child :!label _label_2))
  (`KismetSystemLibrary.PrintString` (`KismetStringLibrary.Conv_DoubleToString` _output_get))
  (if (<= _output_get 0.0)
    (message `/Game/InterfaceAndUI/Interfaces/Interact_Interface.KillPlayer` (`GameplayStatics.GetPlayerController` 0))
    (else
      (`KismetSystemLibrary.Delay` 1.0)
      (if (`self.PlayerInCloseLightBox`)
        (goto _label_2)))))

(event `self.CloseRange.OnComponentEndOverlap`
  (params (OverlappedComponent :type "PrimitiveComponent Object Reference") (OtherActor :type "Actor Object Reference") (OtherComp :type "PrimitiveComponent Object Reference") (OtherBodyIndex :type Integer))
  (cast `/Game/Actors/Characters/AgilityCharacter_Child` OtherActor)
  (set `self.PlayerInCloseLightBox` false))

(event `self.PostProcessAgility.OnComponentActivated`
  (params (Component :type "ActorComponent Object Reference") (bReset :type Boolean)))

(event `self.Box.OnComponentBeginOverlap`
  (params (OverlappedComponent :type "PrimitiveComponent Object Reference") (OtherActor :type "Actor Object Reference") (OtherComp :type "PrimitiveComponent Object Reference") (OtherBodyIndex :type Integer) (bFromSweep :type Boolean) (SweepResult :type "HitResult Structure (by ref)"))
  (cast `/Game/Actors/Characters/AgilityCharacter_Child` OtherActor)
  (set `self.PlayerInLightBox` true)
  (set `self.PlayerInCloseLightBox` true)
  (set `PostProcessComponent.BlendWeight` 1.0 (`self.PostProcessAgility`)))

(event `self.Box.OnComponentEndOverlap`
  (params (OverlappedComponent :type "PrimitiveComponent Object Reference") (OtherActor :type "Actor Object Reference") (OtherComp :type "PrimitiveComponent Object Reference") (OtherBodyIndex :type Integer))
  (cast `/Game/Actors/Characters/AgilityCharacter_Child` OtherActor)
  (set `self.PlayerInLightBox` false)
  (set `self.PlayerInCloseLightBox` false)
  (set `PostProcessComponent.BlendWeight` 0.0 (`self.PostProcessAgility`)))

(fn `UserConstructionScript`)