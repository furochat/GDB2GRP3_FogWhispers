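; Player pawn for the character selection screen, meant to glide between Magnus, Tiago and Mary from the main menu.
; The disconnected logic swaps menu widgets, steps a clamped arrow index behind a CanClick lock, and lerps the pawn to each character's transform through timelines.
; All events are empty and that logic never runs, leaving only an UpdateCharacterName function that re-enables clicking.
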(event `self.ReceiveBeginPlay`)

(event `GoToCharacterSelect`)

(event `GoToTutoSelectCharacter`)

(event `MoveRight`)

(event `MoveLeft`)

(event `PlayerCharacterTimeline`
  (params (Arrow :type Integer)))

(event `UpdateTransform`
  (params (NewTransform :type "Transform Structure") (Alpha :type "Float (double-precision)")))

(event `UpdateCharacterName`
  (params (Count :type Integer)))

(fn `UserConstructionScript`)